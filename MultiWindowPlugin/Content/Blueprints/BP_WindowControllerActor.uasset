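; BP_WindowControllerActor is an actor that routes five window-creation events to indexed window creation.
; On BeginPlay it binds a separate custom event to each of the five Create Window events.
; Each handler calls CreateWindowByIndex with its own fixed window number.
; The CreateWindow event, overlap event and construction script are empty, and Tick is disabled.
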(event Custom|CreateWindow
  (params (Index :type Integer)))

(event Custom|CustomEvent_1
  (Class|WindowControllerActor|CreateWindowbyIndex 2))

(event Custom|CustomEvent_0
  (Class|WindowControllerActor|CreateWindowbyIndex 1))

(event Custom|CustomEvent_2
  (Class|WindowControllerActor|CreateWindowbyIndex 3))

(event Custom|CustomEvent_3
  (Class|WindowControllerActor|CreateWindowbyIndex 4))

(event Custom|CustomEvent_4
  (Class|WindowControllerActor|CreateWindowbyIndex 5))

(event EventBeginPlay
  (EventDispatchers|BindEventtoCreate1Window (delegate Custom|CustomEvent_0))
  (EventDispatchers|BindEventtoCreate2Window (delegate Custom|CustomEvent_1))
  (EventDispatchers|BindEventtoCreate3Window (delegate Custom|CustomEvent_2))
  (EventDispatchers|BindEventtoCreate4Window (delegate Custom|CustomEvent_3))
  (EventDispatchers|BindEventtoCreate5Window (delegate Custom|CustomEvent_4)))

(event Collision|EventActorBeginOverlap
  (params (OtherActor :type Actor%20Object%20Reference)))

(event EventTick
  (params (DeltaSeconds :type Float%20%28single-precision%29)))

(fn ConstructionScript)